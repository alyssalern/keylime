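; KeyLimeMenuGameMode_BP is a game mode Blueprint whose only working logic derives the name of the next numbered level.
; GetNextLevelName reads the last three characters of the current level name as a number, increments it and returns a zero-padded "Level_###" Name.
; It prints both names for debugging and does not load the level itself.
; The event graph, construction script and NewFunction_0 are empty stubs.
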(event EventBeginPlay)

(event EventTick
  (params (DeltaSeconds :type Float%20%28single-precision%29)))

(event EventEndPlay
  (params (EndPlayReason :type EEndPlayReason%20Enum :default "Destroyed")))

(fn ConstructionScript)

(fn NewFunction0)

(fn GetNextLevelName
  (bind _returnvalue (Game|GetCurrentLevelName true))
  (Development|PrintString "MIKO6: current level name: ")
  (Development|PrintString _returnvalue)
  (Development|PrintString ", new level name: ")
  (Development|PrintString (Utilities|String|Append "Level_" (Utilities|String|ToString(Text) (Utilities|Text|ToText(Integer) (+ (Math|Conversions|ToInteger(Byte) (Utilities|String|Right _returnvalue 3)) 1) false true 3 3))))
  (return (Utilities|String|StringToName (Utilities|String|Append "Level_" (Utilities|String|ToString(Text) (Utilities|Text|ToText(Integer) (+ (Math|Conversions|ToInteger(Byte) (Utilities|String|Right _returnvalue 3)) 1) false true 3 3))))))