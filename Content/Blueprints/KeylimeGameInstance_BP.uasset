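; Game instance for Keylime that holds level data and the shared HUD widget.
; On Init it copies every row of the level data table into the LevelDataSet collection.
; It then creates a HUD widget for player controller 0 and stores it, exposed through GetHudUI, without adding it to the viewport here.
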(event EventInit
  (bind _outrownames (DataTable|GetDataTableRowNames "/Game/Data/LevelDataTable.LevelDataTable"))
  (for _array_element _outrownames
    (bind _returnvalue (Utilities|GetDataTableRow "/Game/Data/LevelDataTable.LevelDataTable" _array_element)
      (:then
        (Utilities|Set|Add (Variables|Default|GetLevelDataSet) _returnvalue))))
  (bind _returnvalue_2 (UserInterface|CreateWidget "/Game/Blueprints/UI/HUD_WBP.HUD_WBP_C" (Game|GetPlayerController 0)))
  (Variables|Default|SethudUI _returnvalue_2)
  (Development|PrintString "Created hud ui"))

(fn GetHudUI
  (return (Variables|Default|GethudUI)))