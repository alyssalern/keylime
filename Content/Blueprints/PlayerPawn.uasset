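; Player pawn for Keylime that moves left and right, collects pickups and uses inventory items.
; Touch and action inputs share movement calls, though a right-half touch only stops movement and never starts a rightward move.
; Tick pins the lagged camera rig's height, following the mesh along X, and offsets a hidden-by-default teleport indicator by the game instance's distance.
; Overlaps consume pickups, UseItem triggers the game mode's inventory, and level completion calls OnLevelEnd.
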(event Custom|HandleLevelCompleteEvent
  (Class|PlayerPawn|OnLevelEnd))

(event EventBeginPlay
  (bind _springarm (Variables|Default|GetSpringArm))
  (EventDispatchers|BindEventtoLevelCompleteEvent (delegate Custom|HandleLevelCompleteEvent))
  (Variables|/Script/Engine.SpringArmComponent|SetbEnableCameraLag _springarm true)
  (Variables|/Script/Engine.SpringArmComponent|SetbDrawDebugLagMarkers _springarm false)
  (Variables|/Script/Engine.SpringArmComponent|SetCameraLagSpeed _springarm 2.0)
  (Variables|/Script/Engine.SpringArmComponent|SetCameraLagMaxDistance _springarm 2e+02))

(event EventTick
  (params (DeltaSeconds :type Float%20%28single-precision%29))
  (bind _playersphere (Variables|Default|GetPlayerSphere))
  (bind _camera (Variables|Default|GetCamera))
  (bind _returnvalue (Transformation|GetWorldLocation _playersphere))
  (bind _returnvalue_2 (Transformation|GetWorldLocation _camera))
  (bind (_x _y _z) (Math|Vector|BreakVector _returnvalue))
  (bind (_x_2 _y_2) (Math|Vector|BreakVector _returnvalue_2))
  (Transformation|SetWorldLocation (Variables|Default|GetSpringArm) (Math|Vector|MakeVector (.X (Math|Vector|BreakVector (Transformation|GetWorldLocation (Variables|Default|GetStaticMesh)))) 0.0 4e+02) false true)
  (Transformation|SetWorldLocation (Variables|Default|GetCamera) (Math|Vector|MakeVector _x_2 _y_2 4e+02) false false)
  ;[1 1 1] Place the teleport indicator
  (bind _askeylime_game_instance_bp (Utilities|Casting|CastToKeylimeGameInstance_BP (Game|GetGameInstance)))
  (Transformation|SetWorldLocation (Variables|Default|GetTeleportIndicatorSphere) (Math|Vector|MakeVector (+ (Variables|/Script/KeyLime.KeylimeGameInstance|GetteleportDistance _askeylime_game_instance_bp) _x) _y _z) false false))

(event Collision|EventActorBeginOverlap
  (params (OtherActor :type Actor%20Object%20Reference))
  ;[1 1 1] Collide with Pickup Item
  (bind _aspickup_item (Utilities|Casting|CastToPickupItem OtherActor))
  (if (not (Variables|/Script/KeyLime.PickupItem|GetHasBeenHit _aspickup_item))
    (Class|PickupItem|OnPlayerHit _aspickup_item)
    (Actor|DestroyActor _aspickup_item)))

(event Input|ActionEvents|InputActionUseItem
  (params (Key :type Key%20Structure))
  ;[1 1 1] Use Item
  (:Pressed
    (bind _askey_lime_game_mode_base (Utilities|Casting|CastToKeyLimeGameModeBase (Game|GetGameMode)))
    (Class|Inventory|UseItem (Class|KeyLimeGameModeBase|GetInventory _askey_lime_game_mode_base))))

(event Input|ActionEvents|InputActionMoveLeft
  (params (Key :type Key%20Structure))
  ;[1 1 1] Horizontal movement response to input
  (:Pressed
    (Class|PlayerPawn|OnInputMoveLeft))
  (:Released
    (Class|PlayerPawn|OnInputStopMovingLeft)))

(event Input|ActionEvents|InputActionMoveRight
  (params (Key :type Key%20Structure))
  ;[1 1 1] Horizontal movement response to input
  (:Pressed
    (Class|PlayerPawn|OnInputMoveRight))
  (:Released
    (Class|PlayerPawn|OnInputStopMovingRight)))

(event Input|TouchEvents|InputTouch
  (params (Location :type Vector) (FingerIndex :type ETouchIndex%20Enum))
  (:Pressed
    (switch Utilities|FlowControl|Switch|SwitchonETouchIndex FingerIndex
      (:Touch1
        (if (< (.X (Math|Vector|BreakVector Location)) (/ (.X (Math|Vector2D|BreakVector2D (Viewport|GetViewportSize))) 2.0))
          (Variables|Default|SettouchDownOnLeft true)
          ;[1 1 1] Horizontal movement response to input
          (Class|PlayerPawn|OnInputMoveLeft)
          (else
            (Variables|Default|SettouchDownOnRight true)
            (Class|PlayerPawn|OnInputStopMovingLeft :!label _label))))))
  (:Released
    (switch Utilities|FlowControl|Switch|SwitchonETouchIndex FingerIndex
      (:Touch1
        (if (Variables|Default|GettouchDownOnLeft)
          (Variables|Default|SettouchDownOnLeft false)
          (goto _label)
          (elif (Variables|Default|GettouchDownOnRight)
            (Variables|Default|SettouchDownOnRight false)
            (Class|PlayerPawn|OnInputStopMovingRight)))))))

(fn ConstructionScript
  (Components|Movement|SetUpdatedComponent (Variables|Default|GetProjectileMovement) (Variables|Default|GetPlayerSphere))
  (CallFunction|SetShowTeleportIndicator false))

(fn SetShowTeleportIndicator
  (params (show :type Boolean))
  (Rendering|SetVisibility (Variables|Default|GetTeleportIndicatorSphere) show true))