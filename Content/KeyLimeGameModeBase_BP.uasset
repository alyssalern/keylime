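; Key Lime game mode Blueprint that runs a level's lifecycle, from setup to win or loss.
; BeginPlay shows the game instance's HUD (removed on EndPlay), then finds the LevelDataTable row matching the current level name and broadcasts it.
; Win and lose events notify the player pawn and replace all widgets with the complete or lost screen.
; Winning also stops the level timer and passes the duration to its widget.
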(event Custom|endLevel_Event
  (bind _asplayer_pawn (Utilities|Casting|CastToPlayerPawn (Game|Player|GetPlayerPawn 0)))
  (Default|CallLevelCompleteEvent _asplayer_pawn)
  (bind _returnvalue (UserInterface|CreateWidget "/Game/Blueprints/UI/LevelComplete_WBP.LevelComplete_WBP_C"))
  (Class|KeyLimeGameModeBase|StopLevelTimer)
  (Variables|/Game/Blueprints/UI/LevelComplete_WBP.LevelComplete_WBP_C|SetlevelDurationValue _returnvalue (Class|KeyLimeGameModeBase|GetLevelDuration))
  (Viewport|RemoveAllWidgets)
  (UserInterface|Viewport|AddtoViewport _returnvalue 0))

(event Custom|onLose_Event
  (bind _asplayer_pawn (Utilities|Casting|CastToPlayerPawn (Game|Player|GetPlayerPawn 0)))
  (Class|PlayerPawn|OnTimerExpired _asplayer_pawn)
  (Default|CallLevelCompleteEvent _asplayer_pawn)
  (bind _returnvalue (UserInterface|CreateWidget "/Game/Blueprints/UI/Lost_WBP.Lost_WBP_C"))
  (Viewport|RemoveAllWidgets)
  (UserInterface|Viewport|AddtoViewport _returnvalue 0))

(event EventBeginPlay
  (bind _askeylime_game_instance_bp (Utilities|Casting|CastToKeylimeGameInstance_BP (Game|GetGameInstance)))
  (bind _hudui (Default|GetHudUI _askeylime_game_instance_bp))
  (UserInterface|Viewport|AddtoViewport _hudui 0)
  ;[1 1 1] Set level data
  (bind _outrownames (DataTable|GetDataTableRowNames "/Game/Data/LevelDataTable.LevelDataTable"))
  (bind _array_element (Utilities|Array|ForEachLoopwithBreak _outrownames :!label _label)
    (:LoopBody
      (bind _returnvalue (Utilities|GetDataTableRow "/Game/Data/LevelDataTable.LevelDataTable" _array_element)
        (:then
          (bind _returnvalue_2 (Game|GetCurrentLevelName true))
          (if (Utilities|Enum|Equal(Enum) _returnvalue_2 (.LevelName (Utilities|Struct|BreakLevelStruct _returnvalue)))
            (bind _output_get (Variables|Default|SetlevelData _returnvalue))
            (Development|PrintString "Set level data" true true "(R=0.351907,G=0.064354,B=1.000000,A=1.000000)" 1e+01)
            (Default|CallLevelDataSet _output_get)
            (Development|PrintString "The time from GmaeModeBase is " true true "(R=0.956082,G=0.953415,B=1.000000,A=1.000000)" 1e+01)
            (Development|PrintString (Utilities|String|ToString(Integer) (Class|KismetMathLibrary|GetMilliseconds (.availableTime (Utilities|Struct|BreakLevelStruct _output_get)))) true true "(R=1.000000,G=1.000000,B=1.000000,A=1.000000)" 1e+01)
            (goto _label Break)))))))

(event EventTick
  (params (DeltaSeconds :type Float%20%28single-precision%29)))

(event EventEndPlay
  (params (EndPlayReason :type EEndPlayReason%20Enum :default "Destroyed"))
  (bind _askeylime_game_instance_bp (Utilities|Casting|CastToKeylimeGameInstance_BP (Game|GetGameInstance)))
  (bind _hudui (Default|GetHudUI _askeylime_game_instance_bp))
  (Widget|RemovefromParent _hudui))

(fn ConstructionScript)